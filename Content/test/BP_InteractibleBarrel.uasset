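; BP_InteractibleBarrel is a physics barrel that can be picked up and dropped.
; On BeginPlay it overrides the Cylinder mesh's mass with a random value, so each barrel weighs differently.
; Pickup disables simulation and attaches the root to the given component, keeping its world transform.
; Drop re-enables simulation on the Cylinder and detaches the actor in place.
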(event EventBeginPlay
  (Class|PrimitiveComponent|SetMassOverrideinKg (Variables|Default|GetCylinder) "None" (Math|Random|RandomFloatinRange 1e+02 1e+04) true))

(event EventDrop
  (Physics|SetSimulatePhysics (Variables|Default|GetCylinder) true)
  (Transformation|DetachFromActor "KeepWorld" "KeepWorld" "KeepWorld"))

(event EventPickup
  (params (AttachTo :type Scene%20Component%20Object%20Reference))
  (Physics|SetSimulatePhysics (Variables|Default|GetCylinder) false)
  (Transformation|AttachComponentToComponent (VehicleSound|GetRootComponent) AttachTo "None" "KeepWorld" "KeepWorld" "KeepWorld" false))

(fn ConstructionScript)