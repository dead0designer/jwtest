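; BP_InteractibleSphere is a test physics sphere that can be picked up and dropped.
; On BeginPlay it overrides the sphere's mass with a random value across a wide range.
; Pickup turns off physics simulation and attaches the root component to the given parent, keeping its world transform.
; Drop re-enables physics and detaches the actor in place.
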(event EventBeginPlay
  (Class|PrimitiveComponent|SetMassOverrideinKg (Variables|Default|GetSphere) "None" (Math|Random|RandomFloatinRange 1e+02 1e+04) true))

(event EventPickup
  (params (AttachTo :type Scene%20Component%20Object%20Reference))
  (Physics|SetSimulatePhysics (Variables|Default|GetSphere) false)
  (Transformation|AttachComponentToComponent (VehicleSound|GetRootComponent) AttachTo "None" "KeepWorld" "KeepWorld" "KeepWorld" false))

(event EventDrop
  (Physics|SetSimulatePhysics (Variables|Default|GetSphere) true)
  (Transformation|DetachFromActor "KeepWorld" "KeepWorld" "KeepWorld"))

(fn ConstructionScript)